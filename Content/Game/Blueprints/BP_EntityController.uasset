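; BP_EntityController is a manager actor that supplies entities with target locations based on gameplay tags.
; On BeginPlay it gathers every BP_ClearEnemy into EntityArray and sets itself as their owner.
; IGetNearest maps entities with exactly matching tags by distance to the requester and returns the closest one's location.
; With no tags or no match, it returns a random offset around the requester's position.
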(event `self.ReceiveBeginPlay`
  (bind _outactors (`GameplayStatics.GetAllActorsOfClass` "/Game/Game/Blueprints/Entities/BP_ClearEnemy.BP_ClearEnemy_C"))
  (for _array_element _outactors
    (`self.SetOwner` _array_element self)
    (`KismetArrayLibrary.Array_Add` (`self.EntityArray`) _array_element)))

(fn `AddRandomLocation`
  (params (A :type "Vector Structure"))
  (returns (ReturnValue :type "Vector Structure"))
  (bind _returnvalue (`KismetMathLibrary.RandomFloatInRange` -250.0 250.0))
  (return (+ A (`KismetMathLibrary.MakeVector` _returnvalue _returnvalue _returnvalue))))

(fn `I_GetNearest`
  (params (Type :type "GameplayTagContainer Structure") (Entity :type "/Game/Game/Blueprints/Entities/BP_ClearEnemy Object Reference"))
  (returns (Location :type "Vector Structure"))
  (locals (LocalSuitableEntity :type "Map of Float (double-precision) to /Game/Game/Blueprints/Entities/BP_ClearEnemy Object Reference"))
  (`self.EmptyGT` Type
    (:`True`
      (return (`self.AddRandomLocation` (`self.K2_GetActorLocation` (`local.Entity`)))))
    (:`False`
      (for _array_element (`self.EntityArray`)
        (if (`BlueprintGameplayTagLibrary.MatchesAnyTags` (`/Game/Game/Blueprints/Entities/BP_ClearEnemy.Type` _array_element) (`local.Type`) true)
          (`BlueprintMapLibrary.Map_Add` (`local.LocalSuitableEntity`) (`self.GetDistanceTo` _array_element (`local.Entity`)) _array_element)))
      (if (== (`BlueprintMapLibrary.Map_Length` (`local.LocalSuitableEntity`)) 0)
        (return (`self.AddRandomLocation` (`self.K2_GetActorLocation` (`local.Entity`))))
        (else
          (bind _keys (`BlueprintMapLibrary.Map_Keys` (`local.LocalSuitableEntity`)))
          (return (`self.K2_GetActorLocation` (`BlueprintMapLibrary.Map_Find` (`local.LocalSuitableEntity`) (`.MinValue` (`KismetMathLibrary.MinOfFloatArray` _keys))))))))))

(fn `UserConstructionScript`)