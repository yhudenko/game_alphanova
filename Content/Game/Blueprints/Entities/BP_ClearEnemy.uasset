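; Enemy entity that plays an infection-style tag game, switching behavior on a gameplay tag Type: Clear, Cleaner or Marked.
; After a random start delay, a looping timer asks the owner via interface for the nearest target and impulses toward it.
; Cleaners seek Marked and Marked seek Clear.
; HitAction spreads Marked color to Clear enemies or lets Cleaners restore Marked ones to class-default type and material.
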(event `self.ReceiveBeginPlay`
  (`parent.ReceiveBeginPlay`)
  (`KismetSystemLibrary.Delay` (`KismetMathLibrary.RandomFloatInRange` 0.0 2.0))
  (bind _returnvalue (`KismetSystemLibrary.K2_SetTimerDelegate` (delegate `TurnLoop`) 2.0 true))
  (set `self.Timer` _returnvalue))

(event `TurnLoop`
  (bind _location (message `/Game/Game/Blueprints/BPI_EntityController.I_GetNearest` (`self.GetOwner`) (`self.SelectGT` (struct) (struct :`GameplayTags` (struct :`(TagName` "Entity.Marked"))) (struct :`GameplayTags` (struct :`(TagName` "Entity.Clear"))) (`self.Type`)) self))
  (`self.AddImpulseToDirection` (`KismetMathLibrary.GetDirectionUnitVector` (`self.K2_GetActorLocation`) _location) 10.0 1.5))

(fn `HitAction`
  (params (Enemy :type "/Game/Game/Blueprints/Entities/BP_ClearEnemy Object Reference"))
  (`|SwitchGameplayTag` (`self.Type`)
    (:`Default`
      (return))
    (:`Entity.Cleaner`
      (`self.SetClear` Enemy)
      (return))
    (:`Entity.Marked`
      (`self.SetMarked` Enemy (`self.Color`) false)
      (return))))

(fn `SelectGT`
  (params (Clear :type "GameplayTagContainer Structure") (Cleaner :type "GameplayTagContainer Structure") (Marked :type "GameplayTagContainer Structure") (Index :type "GameplayTag Structure"))
  (returns (ReturnValue :type "GameplayTagContainer Structure"))
  (`|SwitchGameplayTag` Index
    (:`Default`
      (return))
    (:`Entity.Clear`
      (return Clear))
    (:`Entity.Cleaner`
      (return Cleaner))
    (:`Entity.Marked`
      (return Marked))))

(fn `SetClear`
  (bind (_type _timer _color) (defaults `Object` (`GameplayStatics.GetObjectClass` self)))
  (`|SwitchGameplayTag` (`self.Type`)
    (:`Default`
      (return))
    (:`Entity.Marked`
      (set `self.Type` _type)
      (bind _output_get (set `self.Color` _color))
      (`PrimitiveComponent.SetMaterial` (`self.StaticMesh`) 0 _output_get)
      (return))))

(fn `SetMarked`
  (params (Color :type "MaterialInstance Object Reference") (Forced :type Boolean))
  (if (or Forced (`BlueprintGameplayTagLibrary.MatchesTag` (`self.Type`) (struct :`TagName` "Entity.Clear") true))
    (set `self.Type` (struct :`TagName` "Entity.Marked"))
    (bind _output_get (set `self.Color` Color))
    (`PrimitiveComponent.SetMaterial` (`self.StaticMesh`) 0 _output_get)
    (return)
    (else
      (return))))

(fn `UserConstructionScript`
  (`parent.UserConstructionScript`))