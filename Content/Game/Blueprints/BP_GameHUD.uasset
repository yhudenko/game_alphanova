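; BP_GameHUD is the in-game HUD that manages the character widget and a result screen showing time and place.
; On BeginPlay it adds Character_WB to the viewport with game-only input and a hidden cursor, then removes it when destroyed.
; AddResult creates Result_WB and switches to UI-only input with a visible cursor.
; RemoveResult removes that screen and restores game-only input.
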(event `self.ReceiveBeginPlay`
  (bind _returnvalue (`self.GetOwningPlayerController`))
  (bind _returnvalue_2 (`|CreateWidget` "/Game/Game/UI/Character_WB.Character_WB_C" (`self.GetOwningPlayerController`)))
  (bind _output_get (set `self.CharacterWB` _returnvalue_2))
  (`UserWidget.AddToViewport` _output_get 0)
  (set `PlayerController.bShowMouseCursor` false _returnvalue)
  (`WidgetBlueprintLibrary.SetInputMode_GameOnly` _returnvalue))

(event `self.ReceiveDestroyed`
  (`Widget.RemoveFromParent` (`self.CharacterWB`)))

(event `AddResult`
  (params (Time :type "Float (double-precision)") (Place :type Integer))
  (bind _returnvalue (`self.GetOwningPlayerController`))
  (bind _returnvalue_2 (`|CreateWidget` "/Game/Game/UI/Result_WB.Result_WB_C" _returnvalue Time Place))
  (bind _output_get (set `self.ResultWB` _returnvalue_2))
  (`UserWidget.AddToViewport` _output_get 0)
  (set `PlayerController.bShowMouseCursor` true _returnvalue)
  (`WidgetBlueprintLibrary.SetInputMode_UIOnlyEx` _returnvalue (`self.ResultWB`)))

(event `RemoveResult`
  (bind _returnvalue (`self.GetOwningPlayerController`))
  (`Widget.RemoveFromParent` (`self.ResultWB`))
  (set `PlayerController.bShowMouseCursor` false _returnvalue)
  (`WidgetBlueprintLibrary.SetInputMode_GameOnly` _returnvalue))

(fn `UserConstructionScript`)