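; BP_Entity is a physics-driven actor with a configurable mesh and material.
; Its construction script applies the Mesh variable to its static mesh component and, if that succeeds, sets Color as the material.
; AddImpulseToDirection launches it using the direction's X and Y with Trajectory as Z, scaled by the passed multiplier and ForceMulty.
; The event graph holds only disabled placeholder events.
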(fn `AddImpulseToDirection`
  (params (Direction :type "Vector Structure") (Multy :type "Float (double-precision)") (Trajectory :type "Float (double-precision)"))
  (`PrimitiveComponent.AddImpulse` (`self.StaticMesh`) (* (`KismetMathLibrary.MakeVector` (.x Direction) (.y Direction) Trajectory) (* Multy (`self.ForceMulty`))) "None" false)
  (return))

(fn `UserConstructionScript`
  (bind _returnvalue (`StaticMeshComponent.SetStaticMesh` (`self.StaticMesh`) (`self.Mesh`)))
  (if _returnvalue
    (`PrimitiveComponent.SetMaterial` (`self.StaticMesh`) 0 (`self.Color`))))