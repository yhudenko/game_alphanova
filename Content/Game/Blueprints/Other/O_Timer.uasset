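; Reusable timer Blueprint that counts elapsed time and broadcasts it to listeners.
; Start sets a looping timer by function name at the TimeAccuracy interval and stores its handle.
; Each Timer Body tick adds that interval to Time and fires the TimeUpdated event dispatcher with the new total.
; Pause and Clear act on the timer by function name; neither resets Time.
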(event `Start`
  (bind _returnvalue (`KismetSystemLibrary.K2_SetTimer` null "Timer Body" (`self.TimeAccuracy`) true))
  (set `self.TimerHandle` _returnvalue))

(fn `Clear`
  (`KismetSystemLibrary.K2_ClearTimer` null "Timer Body"))

(fn `Pause`
  (`KismetSystemLibrary.K2_PauseTimer` null "Timer Body"))

(fn `Timer Body`
  (bind _output_get (set `self.Time` (+ (`self.Time`) (`self.TimeAccuracy`))))
  (`self.ED_TimeUpdated` _output_get)
  (return))