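; Results save asset that keeps a ranked list of record times with the date each was set.
; SaveResult inserts a new time before the first slower entry, or appends it at the end, keeping the list ascending so lower times rank higher.
; A parallel DateTime array receives the current date at the same index, and the function returns that index as the new result's position.
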(fn `SaveResult`
  (params (Time :type "Float (double-precision)"))
  (returns (ResultIndex :type Integer))
  (locals (LocalAdded :type Boolean))
  (for (_array_element _array_index) (`self.RecordTime`)
    (if (< Time _array_element)
      (`KismetArrayLibrary.Array_Insert` (`self.RecordTime`) Time _array_index)
      (`KismetArrayLibrary.Array_Insert` (`self.DateTime`) (`KismetMathLibrary.Now`) _array_index)
      (return _array_index)))
  (`KismetArrayLibrary.Array_Add` (`self.RecordTime`) Time)
  (bind _returnvalue (`KismetArrayLibrary.Array_Add` (`self.DateTime`) (`KismetMathLibrary.Now`)))
  (return _returnvalue))