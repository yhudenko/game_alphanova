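; BP_MainMenuHUD is the HUD that puts the main menu on screen.
; On BeginPlay it creates a MeinMenu_WB widget for the owning player, adds it to the viewport, shows the mouse cursor and switches to UI-only input focused on the menu.
; When the HUD is destroyed, it removes the widget from its parent.
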(event `self.ReceiveBeginPlay`
  (bind _returnvalue (`self.GetOwningPlayerController`))
  (bind _returnvalue_2 (`|CreateWidget` "/Game/Game/UI/MeinMenu_WB.MeinMenu_WB_C" (`self.GetOwningPlayerController`)))
  (bind _output_get (set `self.MainMenuWB` _returnvalue_2))
  (`UserWidget.AddToViewport` _output_get 0)
  (set `PlayerController.bShowMouseCursor` true _returnvalue)
  (`WidgetBlueprintLibrary.SetInputMode_UIOnlyEx` _returnvalue (`self.MainMenuWB`)))

(event `self.ReceiveDestroyed`
  (`Widget.RemoveFromParent` (`self.MainMenuWB`)))

(fn `UserConstructionScript`)