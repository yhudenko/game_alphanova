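; BP_GameState drives the game flow between main menu, gameplay and result states, switching pawns and HUDs through interface-style events.
; Starting a game applies cleaner and clean entity counts to BP_EntityController, spawns enemies and restarts an O_Timer.
; Showing results disables pawn input, clears enemies, pauses the timer and saves the time asynchronously via SS_Results, then passes time and place to BP_GameHUD.
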(event `self.ReceiveBeginPlay`
  (bind _outactors (`GameplayStatics.GetAllActorsOfClass` "/Game/Game/Blueprints/BP_EntityController.BP_EntityController_C"))
  (set `self.EntityController` (`|GetArrayItem` _outactors))
  (bind _returnvalue (`|GenericCreateObject` "/Game/Game/Blueprints/Other/O_Timer.O_Timer_C"))
  (set `self.Timer` _returnvalue)
  (`self.I_SetMainMenu`))

(event `self.I_StartGame`
  (params (GameSettings :type "/Game/Game/Blueprints/Save/SS_GameSettings Object Reference"))
  (`self.ApplySettings` GameSettings)
  (switch `/Game/Game/Blueprints/Other/E_GameState` (`self.State`)
    (:`NewEnumerator0`
      (`self.SpawnCharacter`)
      (`self.SetGame`))
    (:`NewEnumerator2`
      (`self.SetGame`)
      (`self.EnableInput` (`Controller.K2_GetPawn` (`GameplayStatics.GetPlayerController` 0)) null))))

(event `self.I_SetMainMenu`
  (bind _returnvalue (`GameplayStatics.GetPlayerController` 0))
  (bind _returnvalue_2 (`|SpawnActorFromClass` "/Game/Game/Blueprints/Other/BP_MenuPawn.BP_MenuPawn_C" (`KismetMathLibrary.MakeTransform` (0.0 0.0 200.0)) "Undefined" "MultiplyWithRoot" null null))
  (`Controller.Possess` _returnvalue _returnvalue_2)
  (`PlayerController.ClientSetHUD` _returnvalue "/Game/Game/Blueprints/BP_MainMenuHUD.BP_MainMenuHUD_C")
  (set `self.State` "NewEnumerator0"))

(event `SpawnCharacter`
  (bind _returnvalue (`|SpawnActorFromClass` "/Game/Game/Blueprints/Entities/BP_Character.BP_Character_C" (`KismetMathLibrary.MakeTransform` (0.0 0.0 100.0)) "Undefined" "MultiplyWithRoot" null null))
  (`Controller.Possess` (`GameplayStatics.GetPlayerController` 0) _returnvalue))

(event `SetGame`
  (`|ExecutionSequence`
    (:`then_0`
      (`PlayerController.ClientSetHUD` (`GameplayStatics.GetPlayerController` 0) "/Game/Game/Blueprints/BP_GameHUD.BP_GameHUD_C"))
    (:`then_1`
      (`/Game/Game/Blueprints/BP_EntityController.SpawnEnemy` (`self.EntityController`)))
    (:`then_2`
      (`/Game/Game/Blueprints/Other/O_Timer.Clear` (`self.Timer`))
      (`/Game/Game/Blueprints/Other/O_Timer.Start` (`self.Timer`)))
    (:`then_3`
      (set `self.State` "NewEnumerator1"))))

(event `self.I_ShowResult`
  (switch `/Game/Game/Blueprints/Other/E_GameState` (`self.State`)
    (:`NewEnumerator1`
      (`self.DisableInput` (`Controller.K2_GetPawn` (`GameplayStatics.GetPlayerController` 0)) null)
      (bind _time (`/Game/Game/Blueprints/Other/O_Timer.Pause` (`self.Timer`)))
      (set `self.State` "NewEnumerator2")
      (`/Game/Game/Blueprints/BP_EntityController.ClearEnemy` (`self.EntityController`))
      (bind _returnvalue (`GameplayStatics.CreateSaveGameObject` "/Game/Game/Blueprints/Save/SS_Results.SS_Results_C"))
      (bind _resultindex (`/Game/Game/Blueprints/Save/SS_Results.SaveResult` _returnvalue _time))
      (`AsyncActionHandleSaveGame.AsyncSaveGameToSlot` _returnvalue (`/Game/Game/Blueprints/Save/SS_Results.SlotName` _returnvalue) (`/Game/Game/Blueprints/Save/SS_Results.UserIndex` _returnvalue)
        (:`Completed`
          (bind _asbp_game_hud (cast `/Game/Game/Blueprints/BP_GameHUD` (`PlayerController.GetHUD` (`GameplayStatics.GetPlayerController` 0))))
          (`/Game/Game/Blueprints/BP_GameHUD.AddResult` _asbp_game_hud _time _resultindex))))))

(fn `ApplySettings`
  (params (Settings :type "/Game/Game/Blueprints/Save/SS_GameSettings Object Reference"))
  (`/Engine/EditorBlueprintResources/StandardMacros.IsValid` Settings
    (:`Is Valid`
      (set `/Game/Game/Blueprints/BP_EntityController.CountClearEntity` (`/Game/Game/Blueprints/Save/SS_GameSettings.CleanCount` Settings) (`self.EntityController`))
      (set `/Game/Game/Blueprints/BP_EntityController.CountCleanerEntity` (`/Game/Game/Blueprints/Save/SS_GameSettings.CleanerCount` Settings) (`self.EntityController`))
      (return))
    (:`Is Not Valid`
      (return))))

(fn `I_GetEntityController`
  (returns (Controller :type "/Game/Game/Blueprints/BP_EntityController Object Reference"))
  (return (`self.EntityController`)))

(fn `I_GetTimer`
  (returns (Timer :type "/Game/Game/Blueprints/Other/O_Timer Object Reference"))
  (return (`self.Timer`)))

(fn `UserConstructionScript`)